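; Timeline board actor for the card game that holds event and fate cards and arranges them in a staggered row.
; SortCards moves each card relative to CardPlacementLocation, stepping back along X and up in Z so the cards cascade.
; Each array is laid out in reverse order, with fate cards continuing after the event cards.
; The event graph and construction script contain no logic.
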(fn `SortCards`
  (bind (_returnvalue_x _returnvalue_y _returnvalue_z) (`KismetMathLibrary.BreakVector` (`SceneComponent.K2_GetComponentLocation` (`self.CardPlacementLocation`))))
  (bind (_returnvalue_x_2 _returnvalue_y_2 _returnvalue_z_2) (`KismetMathLibrary.BreakVector` (`SceneComponent.K2_GetComponentLocation` (`self.CardPlacementLocation`))))
  (for (_ _array_index) (`self.EventCards`)
    (bind _ascard_bp (cast `/Game/GameContent/CardGame/Cards/Card_BP` (`|GetArrayItem` (`self.EventCards`) (- (`KismetArrayLibrary.Array_LastIndex` (`self.EventCards`)) _array_index))))
    (`self.K2_SetActorTransform` _ascard_bp (`KismetMathLibrary.MakeTransform` (`KismetMathLibrary.MakeVector` (+ _returnvalue_x_2 (* -30 _array_index)) _returnvalue_y_2 (+ _returnvalue_z_2 (* 5 _array_index)))) false false))
  (for (_ _array_index_2) (`self.FateCards`)
    (bind _ascard_bp_2 (cast `/Game/GameContent/CardGame/Cards/Card_BP` (`|GetArrayItem` (`self.FateCards`) (- (`KismetArrayLibrary.Array_LastIndex` (`self.FateCards`)) _array_index_2))))
    (bind _returnvalue (+ _array_index_2 (`KismetArrayLibrary.Array_Length` (`self.EventCards`))))
    (`self.K2_SetActorTransform` _ascard_bp_2 (`KismetMathLibrary.MakeTransform` (`KismetMathLibrary.MakeVector` (+ _returnvalue_x (* -30 _returnvalue)) _returnvalue_y (+ _returnvalue_z (* 5 _returnvalue)))) false false))
  (return))

(fn `UserConstructionScript`)
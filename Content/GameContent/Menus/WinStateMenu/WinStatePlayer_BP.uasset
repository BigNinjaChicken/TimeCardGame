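; Player pawn or actor for the end-of-match menu that shows the win or lose screen.
; On BeginPlay it reads PlayerWon from the StateInfor_GI game instance and adds either the Win_WG or Lose_WG widget to the viewport.
; The LeaveGameButton input action quits the game.
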(event `InputAction|LeaveGameButton`
  (params (Key :type "Key Structure"))
  (:`Pressed`
    (`KismetSystemLibrary.QuitGame` (`GameplayStatics.GetPlayerController` 0) "Quit")))

(event `self.ReceiveBeginPlay`
  (bind _asstate_infor_gi (cast `/Game/GameContent/CardGame/SavedInfo/StateInfor_GI` (`GameplayStatics.GetGameInstance`)))
  (if (`/Game/GameContent/CardGame/SavedInfo/StateInfor_GI.PlayerWon` _asstate_infor_gi)
    (bind _returnvalue (`|CreateWidget` "/Game/GameContent/Menus/WinStateMenu/Win_WG.Win_WG_C"))
    (`UserWidget.AddToViewport` _returnvalue 0)
    (else
      (bind _returnvalue_2 (`|CreateWidget` "/Game/GameContent/Menus/WinStateMenu/Lose_WG.Lose_WG_C"))
      (`UserWidget.AddToViewport` _returnvalue_2 0))))

(fn `UserConstructionScript`)
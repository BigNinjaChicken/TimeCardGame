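; Basic AI opponent for a timeline card game, with its own card pools and a token that moves along year slots.
; PlayCards uses a random, non-looping MultiGate to spawn a bad card one year ahead of the player or a neutral or good card at its own year.
; Spawned cards are sorted into that Timeline_BP's event or fate lists by interface.
; Token moves are clamped and lockable; AddCards is a stub and MoveFateCards only notifies the GameManager.
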(event `self.ReceiveBeginPlay`
  (bind _returnvalue (`GameplayStatics.GetActorOfClass` "/Game/GameContent/CardGame/GameManager_BP.GameManager_BP_C"))
  (set `self.GameManagerBP` _returnvalue))

(fn `AddCards`
  (params (CardAmount :type Integer))
  (returns (null :type Boolean))
  (return false))

(fn `CreateDeck`
  (returns (Null :type Boolean))
  (`|ExecutionSequence`
    (:`then_0`
      (`KismetArrayLibrary.Array_Add` (`self.GoodCards`) "/Game/GameContent/CardGame/Cards/EventCards/Medicine/MedicineCard_BP.MedicineCard_BP_C")
      (`|ExecutionSequence`
        (:`then_0`
          (`KismetArrayLibrary.Array_Add` (`self.NeutralCards`) "/Game/GameContent/CardGame/Cards/EventCards/SummonForth/SummonForth_BP.SummonForth_BP_C")
          (`|ExecutionSequence`
            (:`then_0`
              (`KismetArrayLibrary.Array_Add` (`self.BadCards`) "/Game/GameContent/CardGame/Cards/FateCards/Disease/Disease_BP.Disease_BP_C")
              (return false))))))))

(fn `CreateTokens`
  (params (Offset :type "Float (double-precision)"))
  (returns (TokenBP :type "Actor Object Reference") (StartingIndex :type Integer))
  (set `self.TokenOffset` Offset)
  (bind _outactors (`GameplayStatics.GetAllActorsOfClass` "/Game/GameContent/CardGame/Board/Timeline_BP.Timeline_BP_C"))
  (bind _returnvalue (`|SpawnActorFromClass` "/Game/GameContent/CardGame/Enemy/BasicEnemyToken_BP.BasicEnemyToken_BP_C" (`KismetMathLibrary.MakeTransform` (`KismetMathLibrary.MakeVector` (+ (`self.TokenOffset`) (.x (.location (`self.GetTransform` (`|GetArrayItem` _outactors))))) (.y (.location (`self.GetTransform` (`|GetArrayItem` _outactors)))) (.z (.location (`self.GetTransform` (`|GetArrayItem` _outactors)))))) "Undefined" "OverrideRootScale" null null))
  (return _returnvalue 0))

(fn `GetToken`
  (returns (Token :type "Actor Object Reference"))
  (return (`self.TokenBP`)))

(fn `GetYearIndex`
  (returns (Index :type Integer))
  (return (`self.YearIndex`)))

(fn `MoveFateCards`
  (`/Game/GameContent/CardGame/GameManager_BP.FinishedActivatingFateCard` (`self.GameManagerBP`))
  (return))

(fn `MoveToken`
  (params (TokenBP :type "Actor Object Reference") (CurrentYearIndex :type Integer) (MoveHowManyYears :type Integer) (MaxYearIndex :type Integer))
  (returns (null :type Boolean))
  (locals (NextYearIndex :type Integer) (CurrentTokenBP :type "Actor Object Reference"))
  (bind _returnvalue (`KismetMathLibrary.Clamp` (+ CurrentYearIndex MoveHowManyYears) 0 MaxYearIndex))
  (if (`self.IsTokenLocked`)
    (return false)
    (else
      (set `local.CurrentTokenBP` TokenBP)
      (set `local.NextYearIndex` _returnvalue)
      (bind _outactors (`GameplayStatics.GetAllActorsOfClass` "/Game/GameContent/CardGame/Board/Timeline_BP.Timeline_BP_C"))
      (`self.K2_SetActorTransform` (`local.CurrentTokenBP`) (`KismetMathLibrary.MakeTransform` (`KismetMathLibrary.MakeVector` (+ (`self.TokenOffset`) (.x (.location (`self.GetTransform` (`|GetArrayItem` _outactors _returnvalue))))) (.y (.location (`self.GetTransform` (`|GetArrayItem` _outactors _returnvalue)))) (.z (.location (`self.GetTransform` (`|GetArrayItem` _outactors _returnvalue)))))) false false)
      (set `self.YearIndex` (`local.NextYearIndex`))
      (return false))))

(fn `PlayCards`
  (bind _outactors (`GameplayStatics.GetAllActorsOfClass` "/Game/GameContent/CardGame/Board/Timeline_BP.Timeline_BP_C"))
  (set `self.TimeLineBP` _outactors)
  (bind _asplayer_bp (cast `/Game/GameContent/CardGame/Player/Player_BP` (`GameplayStatics.GetPlayerPawn` 0)))
  (set `self.PlayerBP` _asplayer_bp)
  (`|MultiGate` true
    (:`Out 0`
      (bind _astimeline_bp (`self.TimeLineBPInRelationToPlayer` 1))
      (`self.PlayRandomCardOfType` (`self.BadCards`) _astimeline_bp))
    (:`Out 1`
      (bind _timelinebp (`self.TimeLineBPInRelationToThisActor` 0))
      (`self.PlayRandomCardOfType` (`self.NeutralCards`) _timelinebp))
    (:`Out 2`
      (bind _timelinebp_2 (`self.TimeLineBPInRelationToThisActor` 0))
      (`self.PlayRandomCardOfType` (`self.GoodCards`) _timelinebp_2)))
  (return))

(fn `PlayRandomCardOfType`
  (params (CardTypeClass :type "Array of Actor Class Reference") (Timeline :type "/Game/GameContent/CardGame/Board/Timeline_BP Object Reference"))
  (locals (SummonedCard :type "Actor Object Reference"))
  (bind _returnvalue (`|SpawnActorFromClass` (`|GetArrayItem` CardTypeClass (`KismetMathLibrary.RandomInteger` (`KismetArrayLibrary.Array_Length` CardTypeClass))) (`SceneComponent.K2_GetComponentToWorld` (`/Game/GameContent/CardGame/Board/Timeline_BP.CardPlacementLocation` Timeline)) "Undefined" "OverrideRootScale" null null))
  (bind _output_get (set `local.SummonedCard` _returnvalue))
  (cast `/Game/GameContent/CardGame/Cards/EventCards/EventCard_IF` _output_get
    (:`then`
      (`KismetArrayLibrary.Array_Add` (`/Game/GameContent/CardGame/Board/Timeline_BP.EventCards` Timeline) (`local.SummonedCard`))
      (`/Game/GameContent/CardGame/Board/Timeline_BP.SortCards` Timeline :!label _label)
      (return))
    (:`CastFailed`
      (cast `/Game/GameContent/CardGame/Cards/FateCards/FateCard_IF` _returnvalue
        (:`then`
          (`KismetArrayLibrary.Array_Add` (`/Game/GameContent/CardGame/Board/Timeline_BP.FateCards` Timeline) (`local.SummonedCard`))
          (goto _label))
        (:`CastFailed`
          (`KismetSystemLibrary.PrintString` "Error: NotCardType"))))))

(fn `SetLockTokenMovement`
  (params (IsTokenLocked :type Boolean))
  (returns (Null :type Boolean))
  (set `self.IsTokenLocked` IsTokenLocked)
  (return false))

(fn `TimeLineBPInRelationToPlayer`
  (params (CardDistance :type Integer))
  (returns (`AsTimeline BP` :type "/Game/GameContent/CardGame/Board/Timeline_BP Object Reference"))
  (bind _astimeline_bp (cast `/Game/GameContent/CardGame/Board/Timeline_BP` (`|GetArrayItem` (`self.TimeLineBP`) (`KismetMathLibrary.Clamp` (+ CardDistance (`/Game/GameContent/CardGame/Player/Player_BP.YearIndex` (`self.PlayerBP`))) 0 (- (`/Game/GameContent/CardGame/GameManager_BP.AmountOfTimeLineYears` (`self.GameManagerBP`)) 1)))))
  (return _astimeline_bp))

(fn `TimeLineBPInRelationToThisActor`
  (params (CardDistance :type Integer))
  (returns (TimelineBP :type "/Game/GameContent/CardGame/Board/Timeline_BP Object Reference"))
  (bind _astimeline_bp (cast `/Game/GameContent/CardGame/Board/Timeline_BP` (`|GetArrayItem` (`self.TimeLineBP`) (`KismetMathLibrary.Clamp` (+ CardDistance (`self.YearIndex`)) 0 (- (`/Game/GameContent/CardGame/GameManager_BP.AmountOfTimeLineYears` (`self.GameManagerBP`)) 1)))))
  (return _astimeline_bp))

(fn `UserConstructionScript`)
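; Game manager for a timeline card game, where a token reaching the final year loses for its owner.
; BeginPlay spawns the row of year actors, then creates player and enemy tokens and decks.
; Turns alternate: advance the token, draw and play cards, then resolve that year's cards.
; Cards resolve one by one via callbacks, events before fates; events are destroyed, while fates return to the timeline afterwards.
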(event `self.ReceiveBeginPlay`
  ;[1 1 1] Assign Player Variable
  (bind _asplayer_bp (cast `/Game/GameContent/CardGame/Player/Player_BP` (`GameplayStatics.GetPlayerPawn` 0)))
  (set `self.PlayerBP` _asplayer_bp)
  (`|ExecutionSequence`
    (:`then_0`
      (bind _returnvalue (`GameplayStatics.GetActorOfClass` "/Game/GameContent/CardGame/Board/TimelineStart.TimelineStart_C"))
      (`self.CreateTimelineActors` (`self.AmountOfTimeLineYears`) (`self.K2_GetActorLocation` _returnvalue)))
    (:`then_1`
      (bind _returnvalue_2 (`GameplayStatics.GetActorOfClass` "/Game/GameContent/CardGame/Enemy/BasicEnemy_BP.BasicEnemy_BP_C"))
      (set `self.EnemyBP` _returnvalue_2)
      (`|ExecutionSequence`
        (:`then_0`
          (bind (_tokenbp _startingindex) (message `/Game/GameContent/CardGame/PlayableCharacter_Interface.CreateTokens` (`self.PlayerBP`) 180.0))
          (set `/Game/GameContent/CardGame/Player/Player_BP.TokenBP` _tokenbp (`self.PlayerBP`))
          (set `/Game/GameContent/CardGame/Player/Player_BP.YearIndex` _startingindex (`self.PlayerBP`)))
        (:`then_1`
          (bind (_tokenbp_2 _startingindex_2) (message `/Game/GameContent/CardGame/PlayableCharacter_Interface.CreateTokens` (`self.EnemyBP`) 300.0))
          (set `/Game/GameContent/CardGame/Enemy/BasicEnemy_BP.TokenBP` _tokenbp_2 (`self.EnemyBP`))
          (set `/Game/GameContent/CardGame/Enemy/BasicEnemy_BP.YearIndex` _startingindex_2 (`self.EnemyBP`)))))
    (:`then_2`
      (message `/Game/GameContent/CardGame/PlayableCharacter_Interface.CreateDeck` (`self.PlayerBP`)))
    (:`then_3`
      (message `/Game/GameContent/CardGame/PlayableCharacter_Interface.CreateDeck` (`self.EnemyBP`)))
    (:`then_4`
      (set `self.FinishedSetup` true))))

(event `StartGame`
  (if (`self.FinishedSetup`)
    (`/Engine/EditorBlueprintResources/StandardMacros.DoOnce` false
      (:`Completed`
        (`self.PlayerTurn`)))))

(event `PlayerTurn`
  (bind _playerbp (`self.PlayerBP`))
  (message `/Game/GameContent/CardGame/PlayableCharacter_Interface.MoveToken` _playerbp (`/Game/GameContent/CardGame/Player/Player_BP.TokenBP` _playerbp) (`/Game/GameContent/CardGame/Player/Player_BP.YearIndex` _playerbp) 1 (- (`self.AmountOfTimeLineYears`) 1))
  (`/Game/GameContent/CardGame/PlayableCharacter_Interface.AddCards` (`self.PlayerBP`) 2)
  (set `/Game/GameContent/CardGame/Player/Player_BP.PlayCardPhase` true (`self.PlayerBP`)))

(event `FinishedPlayingCards`
  (`self.Activate Cards` (`self.PlayerBP`) (`self.EnemyBP`)))

(event `FinishedActivating Cards`
  (params (Activator :type "Actor Object Reference"))
  (bind _asplayer_bp (cast `/Game/GameContent/CardGame/Player/Player_BP` Activator)
    (:`then`
      (if (== (`/Game/GameContent/CardGame/Player/Player_BP.YearIndex` _asplayer_bp) (- (`self.AmountOfTimeLineYears`) 1))
        (bind _asstate_infor_gi (cast `/Game/GameContent/CardGame/SavedInfo/StateInfor_GI` (`GameplayStatics.GetGameInstance`)))
        (set `/Game/GameContent/CardGame/SavedInfo/StateInfor_GI.PlayerWon` false _asstate_infor_gi)
        (`GameplayStatics.OpenLevel` "WinState")
        (else
          (set `/Game/GameContent/CardGame/Player/PlayersTurn_WG.TurnText` "Opponents Turn" (`/Game/GameContent/CardGame/Player/Player_BP.TurnGUI` (`self.PlayerBP`)))
          (`self.EnemyTurn`))))
    (:`CastFailed`
      (bind _asbasic_enemy_bp (cast `/Game/GameContent/CardGame/Enemy/BasicEnemy_BP` Activator))
      (if (== (`/Game/GameContent/CardGame/Enemy/BasicEnemy_BP.YearIndex` _asbasic_enemy_bp) (- (`self.AmountOfTimeLineYears`) 1))
        (bind _asstate_infor_gi_2 (cast `/Game/GameContent/CardGame/SavedInfo/StateInfor_GI` (`GameplayStatics.GetGameInstance`)))
        (set `/Game/GameContent/CardGame/SavedInfo/StateInfor_GI.PlayerWon` true _asstate_infor_gi_2)
        (`GameplayStatics.OpenLevel` "WinState")
        (else
          (set `/Game/GameContent/CardGame/Player/PlayersTurn_WG.TurnText` "Your Turn" (`/Game/GameContent/CardGame/Player/Player_BP.TurnGUI` (`self.PlayerBP`)))
          (`self.PlayerTurn`))))))

(event `EnemyTurn`
  (bind _enemybp (`self.EnemyBP`))
  (message `/Game/GameContent/CardGame/PlayableCharacter_Interface.MoveToken` _enemybp (`/Game/GameContent/CardGame/Enemy/BasicEnemy_BP.TokenBP` _enemybp) (`/Game/GameContent/CardGame/Enemy/BasicEnemy_BP.YearIndex` _enemybp) 1 (- (`self.AmountOfTimeLineYears`) 1))
  (message `/Game/GameContent/CardGame/PlayableCharacter_Interface.AddCards` (`self.EnemyBP`) 2)
  (`/Game/GameContent/CardGame/Enemy/BasicEnemy_BP.PlayCards` (`self.EnemyBP`))
  (`KismetSystemLibrary.Delay` 2.0)
  (`self.Activate Cards` (`self.EnemyBP`) (`self.PlayerBP`)))

(event `Activate Cards`
  (params (Activator :type "Actor Object Reference") (Enemy :type "Actor Object Reference"))
  (bind _activator (`self.Activator`))
  (bind _output_get (set `self.Activator` Activator))
  (set `self.Enemy` Enemy)
  (bind _index (message `/Game/GameContent/CardGame/PlayableCharacter_Interface.GetYearIndex` _output_get))
  (bind _astimeline_bp (cast `/Game/GameContent/CardGame/Board/Timeline_BP` (`|GetArrayItem` (`self.AllTimelineBP`) _index)))
  (bind _eventcards (`/Game/GameContent/CardGame/Board/Timeline_BP.EventCards` _astimeline_bp))
  (if (== (`KismetArrayLibrary.Array_Length` _eventcards) 0)
    (bind _fatecards (`/Game/GameContent/CardGame/Board/Timeline_BP.FateCards` _astimeline_bp))
    (if (== (`KismetArrayLibrary.Array_Length` _fatecards) 0)
      (for _array_element (`self.AllTimelineBP`)
        (bind _astimeline_bp_2 (cast `/Game/GameContent/CardGame/Board/Timeline_BP` _array_element))
        (bind _activatedfatecards (`/Game/GameContent/CardGame/Board/Timeline_BP.ActivatedFateCards` _astimeline_bp_2))
        (for _array_element_2 _activatedfatecards
          (`KismetArrayLibrary.Array_Add` (`/Game/GameContent/CardGame/Board/Timeline_BP.FateCards` _astimeline_bp_2) _array_element_2))
        (`KismetArrayLibrary.Array_Clear` _activatedfatecards))
      (message `/Game/GameContent/CardGame/PlayableCharacter_Interface.SetLockTokenMovement` _activator false)
      (`self.FinishedActivating Cards` _activator)
      (else
        (bind _ascard_bp (cast `/Game/GameContent/CardGame/Cards/Card_BP` (`|GetArrayItem` _fatecards (`KismetArrayLibrary.Array_LastIndex` _fatecards))))
        (bind _output_get_2 (set `self.ActivatedCard` _ascard_bp))
        (`/Game/GameContent/CardGame/Cards/Card_BP.ActivateCard` _output_get_2 (`self.Activator`) self (`self.Enemy`))))
    (else
      (bind _ascard_bp_2 (cast `/Game/GameContent/CardGame/Cards/Card_BP` (`|GetArrayItem` _eventcards (`KismetArrayLibrary.Array_LastIndex` _eventcards))))
      (bind _output_get_3 (set `self.ActivatedCard` _ascard_bp_2))
      (`/Game/GameContent/CardGame/Cards/Card_BP.ActivateCard` _output_get_3 (`self.Activator`) self (`self.Enemy`)))))

(event `FinishedActivatingFateCard`
  (bind _activatedcard (`self.ActivatedCard`))
  (`KismetArrayLibrary.Array_Add` (`/Game/GameContent/CardGame/Board/Timeline_BP.ActivatedFateCards` (stale `Activate Cards` _astimeline_bp)) _activatedcard)
  (`KismetArrayLibrary.Array_RemoveItem` (`/Game/GameContent/CardGame/Board/Timeline_BP.FateCards` (stale `Activate Cards` _astimeline_bp)) _activatedcard)
  (`self.Activate Cards` (`self.Activator`)))

(event `FinishedActivatingEventCard`
  (bind _activatedcard (`self.ActivatedCard`))
  (`KismetArrayLibrary.Array_RemoveItem` (`/Game/GameContent/CardGame/Board/Timeline_BP.EventCards` (stale `Activate Cards` _astimeline_bp)) _activatedcard)
  (`self.K2_DestroyActor` _activatedcard)
  (`self.Activate Cards` (`self.Activator`)))

(fn `CreateTimelineActors`
  (params (AmountOfYears :type Integer) (StartingWorldLocation :type "Vector Structure"))
  (locals (Offset :type "Float (double-precision)" :default -155.0) (Index :type Integer) (NewTimelineActor :type "/Game/GameContent/CardGame/Board/Timeline_BP Object Reference"))
  (`KismetArrayLibrary.Array_Clear` (`self.AllTimelineBP`))
  (for _index (range AmountOfYears)
    (set `local.Index` _index)
    (bind _returnvalue (`|SpawnActorFromClass` "/Game/GameContent/CardGame/Board/Timeline_BP.Timeline_BP_C" (`KismetMathLibrary.MakeTransform` (`KismetMathLibrary.MakeVector` (.x StartingWorldLocation) (+ (.y StartingWorldLocation) (* (`local.Index`) (`local.Offset`))) (.z StartingWorldLocation))) "Undefined" "OverrideRootScale" null null))
    (bind _output_get (set `local.NewTimelineActor` _returnvalue))
    (`TextRenderComponent.K2_SetText` (`/Game/GameContent/CardGame/Board/Timeline_BP.TextRender` _output_get) (`KismetTextLibrary.Conv_IntToText` (`local.Index`)))
    (`KismetArrayLibrary.Array_Add` (`self.AllTimelineBP`) (`local.NewTimelineActor`))))

(fn `UserConstructionScript`)